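; Functional test that checks whether an ammo pickup's rounds fit within the character weapon's maximum ammo.
; PrepareTest caches the weapon from the referenced Character.
; StartTest converts the Pickup's clips to rounds, adds clip and current ammo, and passes if the total is within max, printing the remaining headroom as "Ammo added".
; It only does the arithmetic and never applies the pickup.
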(event `self.ReceivePrepareTest`
  (set `self.Weapon` (`ShooterCharacter.GetWeapon` (`self.Character`))))

(event `self.ReceiveStartTest`
  (bind _weapon (`self.Weapon`))
  (bind _returnvalue (`ShooterWeapon.GetMaxAmmo` _weapon))
  (bind _returnvalue_2 (+ (`ShooterWeapon.GetCurrentAmmoInClip` _weapon) (+ (* (`ShooterPickup_Ammo.AmmoClips` (`self.Pickup`)) (`ShooterWeapon.GetAmmoPerClip` _weapon)) (`ShooterWeapon.GetCurrentAmmo` _weapon))))
  (if (<= _returnvalue_2 _returnvalue)
    (`KismetSystemLibrary.PrintString` (`KismetStringLibrary.Concat_StrStr` "Ammo added " (`KismetStringLibrary.Conv_IntToString` (- _returnvalue _returnvalue_2))))
    (`self.FinishTest` "Succeeded" "Added ammo to weapon")
    (else
      (`self.FinishTest` "Failed" "Didnt give any ammo"))))

(fn `UserConstructionScript`)