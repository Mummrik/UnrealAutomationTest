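; BP_WeaponTypeTest is a functional test that checks whether an ammo pickup matches the type of the character's weapon.
; PrepareTest caches the weapon from the referenced Character.
; StartTest compares the Pickup's WeaponType to that weapon's class and finishes as Succeeded on a match or Failed otherwise, with a message for each result.
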(event `self.ReceivePrepareTest`
  (set `self.Weapon` (`ShooterCharacter.GetWeapon` (`self.Character`))))

(event `self.ReceiveStartTest`
  (if (== (`ShooterPickup_Ammo.WeaponType` (`self.Pickup`)) (`GameplayStatics.GetObjectClass` (`self.Weapon`)))
    (`self.FinishTest` "Succeeded" "Ammo is for right type")
    (else
      (`self.FinishTest` "Failed" "Ammo is for an other type"))))

(fn `UserConstructionScript`)