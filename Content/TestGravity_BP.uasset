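; Functional test that checks whether a referenced Actor moves down under gravity.
; PrepareTest records the Actor's starting location, then Tick passes the test once its Z drops below that start height plus Threshold.
; An invalid Actor fails the test in either event.
; The graph has no other failure path.
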(event `self.ReceivePrepareTest`
  (bind _actor (`self.Actor`)
    (:`then`
      (set `self.StartingLocation` (`self.K2_GetActorLocation` _actor)))
    (:`else`
      (`self.FinishTest` "Failed" "Actor missing" :!label _label))))

(event `self.ReceiveTick`
  (params (DeltaSeconds :type "Float (single-precision)"))
  (bind (_startinglocation_x _startinglocation_y _startinglocation_z) (`KismetMathLibrary.BreakVector` (`self.StartingLocation`)))
  (bind _actor (`self.Actor`)
    (:`then`
      (bind (_returnvalue_x _returnvalue_y _returnvalue_z) (`KismetMathLibrary.BreakVector` (`self.K2_GetActorLocation` _actor)))
      (if (< _returnvalue_z (+ _startinglocation_z (`self.Threshold`)))
        (`self.FinishTest` "Succeeded" "coool")))
    (:`else`
      (goto _label))))

(fn `UserConstructionScript`)